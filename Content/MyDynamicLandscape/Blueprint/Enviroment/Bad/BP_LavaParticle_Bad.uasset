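; BP_LavaParticle_Bad is a lava particle actor, apparently the "bad" demo variant, that turns into a voxel when frozen.
; Freeze runs once, spawning a half-scale BP_Voxel_Demo near the CollisionMesh location, then destroying the particle.
; The spawn position uses hardcoded 50-unit grid arithmetic with half-cell offsets, noted as needing dynamic determination.
; DemoBindFreeze registers an event with the passed Vulcan's demo freeze binding.
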(event `Freeze`
  (bind (_x _y _z) (`KismetMathLibrary.BreakVector3f` (`SceneComponent.K2_GetComponentLocation` (`self.CollisionMesh`))))
  (`/Engine/EditorBlueprintResources/StandardMacros.DoOnce` false
    (:`Completed`
      (`|SpawnActorFromClass` "/Game/MyDynamicLandscape/Blueprint/Enviroment/BP_Voxel_Demo.BP_Voxel_Demo_C" (`KismetMathLibrary.MakeTransform` (`KismetMathLibrary.MakeVector` (+ (* (/ _x 50) 50) -25.0) (+ (* (/ _y 50) 50) -25.0) (+ (* (/ _z 50) 50) 25.0)) (struct) (0.5 0.5 0.5)) "Undefined" "OverrideRootScale" null null)
      (`self.K2_DestroyActor`))))

(fn `DemoBindFreeze`
  (params (Vulcan :type "/Game/MyDynamicLandscape/Blueprint/Enviroment/Bad/BP_Vulcan_Bad Object Reference"))
  ;[1 0 0.1099] Заморозка для демонстрации
  (add `/Game/MyDynamicLandscape/Blueprint/Enviroment/Bad/BP_Vulcan_Bad.For Demo Bad Freeze` Vulcan (`|CreateDelegate` :!event `Freeze`)))

(fn `UserConstructionScript`)