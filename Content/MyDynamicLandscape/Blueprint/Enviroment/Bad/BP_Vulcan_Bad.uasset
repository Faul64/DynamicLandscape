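; BP_Vulcan_Bad is a volcano actor, marked as the "Bad" variant, that emits lava as individual BP_LavaParticle_Bad actors.
; On BeginPlay a Delay loop spawns particles at StartFlowDirection until the count limit, launching each with a random-strength forward impulse on its collision mesh.
; Each particle binds to the volcano for a demo freeze, but the freeze call here is unconnected.
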(event `self.ReceiveBeginPlay`
  (bind _startflowdirection (`self.StartFlowDirection`))
  (bind (_x _y) (`KismetMathLibrary.BreakVector2D` (`self.StartVelocityRange`)))
  ;[1 1 1] 1000 не предел, просадки только во время спауна
  ;;[1 1 1] SpawnLava
  (if (< (`self.Count`) (`self.NumberParticlesCreate`)) :!label _label
    (bind _returnvalue (`|SpawnActorFromClass` "/Game/MyDynamicLandscape/Blueprint/Enviroment/Bad/BP_LavaParticle_Bad.BP_LavaParticle_Bad_C" (`KismetMathLibrary.MakeTransform` (`SceneComponent.K2_GetComponentLocation` _startflowdirection) (`SceneComponent.K2_GetComponentRotation` _startflowdirection)) "Undefined" "OverrideRootScale" null null))
    (`self.FSetSpawnParametr` _returnvalue)
    (`PrimitiveComponent.AddImpulse` (`LavaParticle.CollisionMesh` _returnvalue) (* (* (`SceneComponent.GetForwardVector` (`self.StartFlowDirection`)) (`KismetMathLibrary.RandomFloatInRange` _x _y)) 100) "None" false)
    (`/Engine/EditorBlueprintResources/StandardMacros.IncrementInt` (`self.Count`)
      (:`  `
        (`KismetSystemLibrary.Delay` (`self.MainDeltaTime`))
        (goto _label)))
    (else
      (`KismetSystemLibrary.Delay` 1.0))))

(fn `FSetSpawnParametr`
  (params (pParticle :type "/Game/MyDynamicLandscape/Blueprint/Enviroment/Bad/BP_LavaParticle_Bad Object Reference"))
  (`/Game/MyDynamicLandscape/Blueprint/Enviroment/Bad/BP_LavaParticle_Bad.DemoBindFreeze` pParticle self))

(fn `UserConstructionScript`)