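; BP_Vulcan_Demo is a demo volcano that spawns one lava particle at StartFlowDirection and moves it with hand-written gravity integration.
; After a start delay, a timer fires Test, which loops through FUpdateVelocity, FUpdateLocation and a one-second Delay.
; Velocity is the particle's GetVelocity plus constant gravity, and location advances via SetActorLocation without sweep.
; Spawn parameters, force update and Tick are empty or disconnected stubs.
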(event `Test`
  (`self.FUpdateVelocity` :!label _label)
  (`self.FUpdateLocation` (`self.Particl`))
  (`KismetSystemLibrary.Delay` 1.0)
  (goto _label))

(event `self.ReceiveBeginPlay`
  (`KismetSystemLibrary.K2_SetTimerDelegate` (delegate `Test`) 2.0)
  (bind _returnvalue (`|SpawnActorFromClass` "/Game/MyDynamicLandscape/Blueprint/Enviroment/BP_LavaParticle_Demo.BP_LavaParticle_Demo_C" (`KismetMathLibrary.MakeTransform` (`SceneComponent.K2_GetComponentLocation` (`self.StartFlowDirection`)) (`SceneComponent.K2_GetComponentRotation` (`self.StartFlowDirection`))) "Undefined" "OverrideRootScale" null null))
  (bind _output_get (set `self.Particl` _returnvalue))
  ;[1 1 1] Comment
  (`self.FSetSpawnParametr` _output_get))

(event `self.ReceiveTick`
  (params (DeltaSeconds :type "Float (single-precision)"))
  ;[1 1 1] 0.008
)

(fn `FSetSpawnParametr`
  (params (PArticle :type "LavaParticle Object Reference")))

(fn `FUpdateForce `
  ;[1 1 1] Обновляем значение сил, действующих на частицу
)

(fn `FUpdateLocation`
  (params (pParticle :type "LavaParticle Object Reference") (dt :type "Float (double-precision)" :default 1.0))
  (bind _dt (`local.dt`))
  (bind _pparticle (`local.pParticle`))
  ;[1 0.8925 0] НА ++ не работает почему-то
  (`self.K2_SetActorLocation` (`local.pParticle`) (+ (`self.K2_GetActorLocation` _pparticle) (* (`LavaParticle.Velocity` _pparticle) (`KismetMathLibrary.MakeVector` _dt _dt _dt))) false false))

(fn `FUpdateVelocity`
  (bind _particl (`self.Particl`))
  (set `LavaParticle.Velocity` (+ (`self.GetVelocity` _particl) (0.0 0.0 0.0) (`self.Const_GravityForce`)) _particl))

(fn `UserConstructionScript`)